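; BP_ShrekClub is a Mordhau club weapon that drives a MusicalWeapon from attack start, attack stop and hits on characters.
; Its construction script scales Release by ReleaseMultiplier across stab, couch and strike attack infos, explicitly reassigning only StabAttack.
; Where cosmetic events run, it also adds an audio component for MusicalWeapon setup.
; SetDistortionEnabled toggles distortion by bypassing the first entry in the sound's source effect chain.
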(event `self.OnAttackStarted`
  (params (Move :type "EAttackMove Enum" :default "RightStrike") (Angle :type "Float (single-precision)"))
  (`/ShrekClub/Components/MusicalWeapon.OnAttackStarted` (`self.MusicalWeapon`)))

(event `self.OnAttackStopped`
  (`/ShrekClub/Components/MusicalWeapon.OnAttackStopped` (`self.MusicalWeapon`)))

(event `self.OnHit`
  (params (Actor :type "Actor Object Reference") (Move :type "EAttackMove Enum" :default "RightStrike") (Bone :type Name) (WorldLocation :type "Vector Structure (by ref)") (Tier :type Byte) (SurfaceType :type Byte))
  ;[1 1 1] Check target is character
  (if (`KismetMathLibrary.ClassIsChildOf` (`GameplayStatics.GetObjectClass` Actor) "/Game/Mordhau/Blueprints/Characters/BP_MordhauCharacter.BP_MordhauCharacter_C")
    (`/ShrekClub/Components/MusicalWeapon.OnEnemyHit` (`self.MusicalWeapon`))))

(fn `ModifyAttackInfo`
  (params (StructRef :type "AttackInfo Structure (by ref)"))
  (returns (StructOut :type "AttackInfo Structure"))
  (bind _structout (setmembers `AttackInfo` :`StructRef` StructRef :`Release` (* (`.Release` (break `AttackInfo` StructRef)) (`self.ReleaseMultiplier`))))
  (return _structout))

(fn `SetDistortionEnabled`
  (params (IsEnabled :type Boolean))
  (bind _output_get (set `self.IsDistorted` IsEnabled))
  (`AudioMixerBlueprintLibrary.SetBypassSourceEffectChainEntry` (`AudioComponent.SourceEffectChain` (`self.SoundSource`)) 0 (not _output_get)))

(fn `UserConstructionScript`
  (`parent.UserConstructionScript`)
  (`|ExecutionSequence`
    (:`then_0`
      (bind _structout (`self.ModifyAttackInfo` (`self.StabAttack`)))
      (set `self.StabAttack` _structout))
    (:`then_1`
      (bind _structout_2 (`self.ModifyAttackInfo` (`self.SecondStabAttack`))))
    (:`then_2`
      (bind _structout_3 (`self.ModifyAttackInfo` (`self.CouchAttack`))))
    (:`then_3`
      (bind _structout_4 (`self.ModifyAttackInfo` (`self.SecondCouchAttack`))))
    (:`then_4`
      (bind _structout_5 (`self.ModifyAttackInfo` (`self.StrikeAttack`))))
    (:`then_5`
      (bind _structout_6 (`self.ModifyAttackInfo` (`self.SecondStrikeAttack`))))
    (:`then_6`
      (`/Engine/EditorBlueprintResources/StandardMacros.Can Execute Cosmetic Events`
        (:`True`
          (bind _returnvalue (`AddComponent|NODE_AddAudioComponent-2`))
          (`/ShrekClub/Components/MusicalWeapon.Setup` (`self.MusicalWeapon`) _returnvalue))))))